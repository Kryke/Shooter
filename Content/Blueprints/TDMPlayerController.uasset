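; Player controller for team deathmatch that handles a player's lobby, team choice, kill and death counts, and match UI.
; On begin play it possesses a StartGameView actor with authority and creates the lobby and HUD widgets for switching between lobby and match.
; Stat and server-refresh events call TDMGameMode, while other events fill the scoreboard, player lists and end-game banner.
; Team selection passes through a server event to a multicast.
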(event `ClearScoreboard`
  ;[0.3904 1 0.4224] Scoreboard
  (`/Game/UI/Scoreboard/ScoreBoard.Clear` (`/Game/UI/HUD/UMG_PlayerHUD.ScoreBoard` (`self.HUDWIdget`))))

(event `Addkill`
  (params (Team :type Integer))
  ;[0.3904 1 0.4224] Scoreboard
  (`/Engine/EditorBlueprintResources/StandardMacros.IncrementInt` (`self.Kills`)
    (:`  `
      (bind _astdmgame_mode (cast `/Game/Blueprints/TDMGameMode` (`GameplayStatics.GetGameMode`)))
      (`/Game/Blueprints/TDMGameMode.UpdateScoreboard` _astdmgame_mode)
      (`/Game/Blueprints/TDMGameMode.UpdateScore` _astdmgame_mode Team))))

(event `AddDeath`
  ;[0.3904 1 0.4224] Scoreboard
  (`/Engine/EditorBlueprintResources/StandardMacros.IncrementInt` (`self.Deaths`)
    (:`  `
      (bind _astdmgame_mode (cast `/Game/Blueprints/TDMGameMode` (`GameplayStatics.GetGameMode`)))
      (`/Game/Blueprints/TDMGameMode.UpdateScoreboard` _astdmgame_mode))))

(event `AddPlayerToSCoreboard`
  (params (IsOwnPlayer :type Boolean) (Name :type String) (Kills :type Integer) (Deaths :type Integer) (Position :type Integer) (Team :type Integer))
  ;[0.3904 1 0.4224] Scoreboard
  (`/Game/UI/Scoreboard/ScoreBoard.AddPlayerOnTeam` (`/Game/UI/HUD/UMG_PlayerHUD.ScoreBoard` (`self.HUDWIdget`)) IsOwnPlayer Name Kills Deaths Position Team))

(event `UpdateSCore`
  (params (Kills :type Integer) (Team :type Integer) (IsWon :type Boolean) (Rounds :type Integer))
  ;[0.3904 1 0.4224] Scoreboard
  (`/Game/UI/HUD/UMG_PlayerHUD.UpdateTeamScore` (`self.HUDWIdget`) Kills Team IsWon Rounds))

(event `ShowLobbyWidget`
  ;[0.3904 1 0.4224] Scoreboard
  (`UserWidget.AddToViewport` (`self.LobbyWidget`) 0)
  (`Widget.RemoveFromParent` (`self.HUDWIdget`))
  (bind _outactors (`GameplayStatics.GetAllActorsOfClass` "/Game/Blueprints/StartGameView.StartGameView_C"))
  (`self.Possess` (`|GetArrayItem` _outactors))
  (set `self.bShowMouseCursor` true)
  (`self.UpdateServerFromPC`))

(event `ShowEndGameWidget`
  (params (EndGameWinLoseText :type String) (Winner :type Integer))
  ;[0.3904 1 0.4224] Scoreboard
  (bind _returnvalue (`|CreateWidget` "/Game/UI/Gameplay/UMG_EndGameWidget.UMG_EndGameWidget_C" null EndGameWinLoseText (make `SlateColor` (`KismetMathLibrary.SelectColor` (struct :`G` 1.0 :`B` 0.000452 :`A` 1.0) (struct :`R` 1.0 :`B` 0.018015 :`A` 1.0) (== Winner (`self.SelectedTeam`))))))
  (bind _output_get (set `self.EndGameWidget` _returnvalue))
  (`UserWidget.AddToViewport` _returnvalue 0)
  (`UserWidget.AddToViewport` _output_get 0)
  (`KismetSystemLibrary.Delay` 3.0)
  (`Widget.RemoveFromParent` (`self.EndGameWidget`)))

(event `UpdateServerData`
  (params (ServerMap :type Text) (ServerName :type Text) (ServerSlots :type Integer))
  (bind _lobbywidget (`self.LobbyWidget`))
  ;[1 0.8851 0.4842] Update Server Data
  (set `/Game/UI/Lobby/UMG_TeamSelection.ServerMap` ServerMap _lobbywidget)
  (set `/Game/UI/Lobby/UMG_TeamSelection.ServerName` ServerName _lobbywidget)
  (set `/Game/UI/Lobby/UMG_TeamSelection.ServerSlots` ServerSlots _lobbywidget))

(event `KickPlayer`
  ;[1 0.2708 0.2708] PlayerList
  (`GameplayStatics.OpenLevel` "MainMenu")
  (`DestroySessionCallbackProxy.DestroySession` self))

(event `ClearPlayerList`
  ;[1 0.2708 0.2708] PlayerList
  (`/Game/UI/Lobby/UMG_TeamSelection.ClearList` (`self.LobbyWidget`)))

(event `UpdateNumberOfPlayers`
  (params (CurrentSlots :type Integer))
  ;[1 0.8851 0.4842] Update Server Data
  (set `/Game/UI/Lobby/UMG_TeamSelection.CurrentSlots` CurrentSlots (`self.LobbyWidget`)))

(event `AddPlayerToMainList`
  (params (isFail :type Boolean) (PlayerName :type Text) (ProfileImage :type "Texture2D Object Reference") (PlayerIndex :type Integer) (TeamColor :type "LinearColor Structure"))
  ;[1 0.2708 0.2708] PlayerList
  (bind _returnvalue (`|CreateWidget` "/Game/UI/Lobby/UMG_LobbyPlayerSlor.UMG_LobbyPlayerSlor_C" self isFail PlayerName ProfileImage PlayerIndex TeamColor))
  (`PanelWidget.AddChild` (`/Game/UI/Lobby/UMG_TeamSelection.AllPlayersList` (`self.LobbyWidget`)) _returnvalue))

(event `Loading`
  ;[1 0.5782 0.3229] Loading
  (`Widget.RemoveFromParent` (`self.LobbyWidget`))
  (set `self.bShowMouseCursor` false)
  (`UserWidget.AddToViewport` (`self.HUDWIdget`) 0))

(event `AddPlayerToTeamOne`
  (params (isFail :type Boolean) (PlayerName :type Text) (ProfileImage :type "Texture2D Object Reference") (PlayerIndex :type Integer) (TeamColor :type "LinearColor Structure"))
  (bind _lobbywidget (`self.LobbyWidget`))
  ;[1 0.2708 0.2708] PlayerList
  (bind _returnvalue (`|CreateWidget` "/Game/UI/Lobby/UMG_LobbyPlayerSlor.UMG_LobbyPlayerSlor_C" self isFail PlayerName ProfileImage PlayerIndex TeamColor))
  (`PanelWidget.AddChild` (`/Game/UI/Lobby/UMG_TeamSelection.TeamOneList` _lobbywidget) _returnvalue)
  (`/Engine/EditorBlueprintResources/StandardMacros.IncrementInt` (`/Game/UI/Lobby/UMG_TeamSelection.TeamOneCurrentPlayers` _lobbywidget)))

(event `AddPlayerToTeamTwo`
  (params (isFail :type Boolean) (PlayerName :type Text) (ProfileImage :type "Texture2D Object Reference") (PlayerIndex :type Integer) (TeamColor :type "LinearColor Structure"))
  (bind _lobbywidget (`self.LobbyWidget`))
  ;[1 0.2708 0.2708] PlayerList
  (bind _returnvalue (`|CreateWidget` "/Game/UI/Lobby/UMG_LobbyPlayerSlor.UMG_LobbyPlayerSlor_C" self isFail PlayerName ProfileImage PlayerIndex TeamColor))
  (`PanelWidget.AddChild` (`/Game/UI/Lobby/UMG_TeamSelection.TeamTwoList` _lobbywidget) _returnvalue)
  (`/Engine/EditorBlueprintResources/StandardMacros.IncrementInt` (`/Game/UI/Lobby/UMG_TeamSelection.TeamTwoCurrentPlayers` _lobbywidget)))

(event `Join/LeaveTeamMulticast`
  (params (Team :type Integer))
  ;[1 0.2708 0.2708] PlayerList
  (set `self.SelectedTeam` Team))

(event `UpdateServerFromPC`
  ;[1 0.2708 0.2708] PlayerList
  (bind _astdmgame_mode (cast `/Game/Blueprints/TDMGameMode` (`GameplayStatics.GetGameMode`)))
  (`/Game/Blueprints/TDMGameMode.UpdateServer` _astdmgame_mode))

(event `SetTeamNumberforWIdget`
  (params (Team :type Integer))
  ;[1 0.2708 0.2708] PlayerList
  (set `/Game/UI/Lobby/UMG_TeamSelection.TEamNumber&` Team (`self.LobbyWidget`)))

(event `UpdateGameStatsFromPC`
  ;[1 0.2708 0.2708] PlayerList
  (bind _astdmgame_mode (cast `/Game/Blueprints/TDMGameMode` (`GameplayStatics.GetGameMode`)))
  (switch `int` (`self.SelectedTeam`)
    (:`1`
      (`/Engine/EditorBlueprintResources/StandardMacros.IncrementInt` (`/Game/Blueprints/TDMGameMode.TeamOneKillsNumber` _astdmgame_mode)))
    (:`2`
      (`/Engine/EditorBlueprintResources/StandardMacros.IncrementInt` (`/Game/Blueprints/TDMGameMode.TeamTwoKillsNumber` _astdmgame_mode)))))

(event `Join/LeaveTeamServer`
  (params (Team :type Integer))
  ;[1 0.2708 0.2708] PlayerList
  (`self.Join/LeaveTeamMulticast` Team))

(event `self.ReceiveBeginPlay`
  ;[0.4518 0.6452 1] Begin
  (`|ExecutionSequence`
    (:`then_0`
      (`/Engine/EditorBlueprintResources/ActorMacros.Switch Has Authority`
        (:`Authority`
          (bind _outactors (`GameplayStatics.GetAllActorsOfClass` "/Game/Blueprints/StartGameView.StartGameView_C"))
          (`self.Possess` (`|GetArrayItem` _outactors)))))
    (:`then_1`
      (if (`self.IsLocalController`)
        (bind _returnvalue (`|CreateWidget` "/Game/UI/Lobby/UMG_TeamSelection.UMG_TeamSelection_C" null "" "" (`self.CurrentSession`)))
        (bind _output_get (set `self.LobbyWidget` _returnvalue))
        (`UserWidget.AddToViewport` _output_get 0)
        (`Widget.SetVisibility` _output_get "Hidden")
        (set `self.bShowMouseCursor` true)
        (`KismetSystemLibrary.Delay` 0.75)
        (`Widget.SetVisibility` _output_get "Visible")))
    (:`then_2`
      (bind _returnvalue_2 (`|CreateWidget` "/Game/UI/HUD/UMG_PlayerHUD.UMG_PlayerHUD_C"))
      (set `self.HUDWIdget` _returnvalue_2))))

(fn `UserConstructionScript`)