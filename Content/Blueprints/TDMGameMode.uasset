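; Team deathmatch game mode that runs the lobby, team spawning, scoring and round flow.
; Logins update a controller list, enforcing the slot limit from MainGameInstance and pushing team lists with Steam avatars to every player.
; JoinGame possesses team characters at random spawns, and a kill-sorted scoreboard is rebuilt per client.
; Reaching the kill limit wins a round and repositions players; two round wins reset stats and return everyone to the lobby.
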(event `UpdateScoreboard`
  (bind _indexofmaxvalue (`KismetMathLibrary.MaxOfIntArray` (`self.Kills`)))
  ;[0.09783 1 0.5293] Scoreboard
  ;;[0.06314 1 0.3466] Clear All Data
  (`KismetArrayLibrary.Array_Clear` (`self.PlayersAddedToScoreboard`))
  (`KismetArrayLibrary.Array_Clear` (`self.Copies`))
  (`KismetArrayLibrary.Array_Clear` (`self.Kills`))
  ;;[0.06314 1 0.3466] Get Kill Data
  (bind _output_get (set `self.Copies` (`self.PCs`)))
  (for _array_element _output_get
    (bind _astdmplayer_controller (cast `/Game/Blueprints/TDMPlayerController` _array_element))
    (`KismetArrayLibrary.Array_Add` (`self.Kills`) (`/Game/Blueprints/TDMPlayerController.Kills` _astdmplayer_controller)))
  ;;[0.06314 1 0.3466] Sort Player By Kills
  (while (> (`KismetArrayLibrary.Array_Length` (`self.Kills`)) 0)
    (`KismetArrayLibrary.Array_Add` (`self.PlayersAddedToScoreboard`) (`|GetArrayItem` (`self.Copies`) _indexofmaxvalue))
    (`KismetArrayLibrary.Array_Remove` (`self.Copies`) _indexofmaxvalue)
    (`KismetArrayLibrary.Array_Remove` (`self.Kills`) _indexofmaxvalue))
  ;;[0.06314 1 0.3466] Add Players To Scoreboard
  (for _array_element_2 (`self.PCs`)
    (bind _astdmplayer_controller_2 (cast `/Game/Blueprints/TDMPlayerController` _array_element_2))
    (set `self.TeamOnePlayerPlacement` 0)
    (set `self.TeamTwoPlayerPlacement` 0)
    (`/Game/Blueprints/TDMPlayerController.ClearScoreboard` _astdmplayer_controller_2)
    (for _array_element_3 (`self.PlayersAddedToScoreboard`)
      (bind _astdmplayer_controller_3 (cast `/Game/Blueprints/TDMPlayerController` _array_element_3))
      (switch `int` (`/Game/Blueprints/TDMPlayerController.SelectedTeam` _astdmplayer_controller_3)
        (:`1`
          (bind _result (`/Engine/EditorBlueprintResources/StandardMacros.IncrementInt` (`self.TeamOnePlayerPlacement`))
            (:`  `
              (set `self.Temp Position` _result))))
        (:`2`
          (bind _result_2 (`/Engine/EditorBlueprintResources/StandardMacros.IncrementInt` (`self.TeamTwoPlayerPlacement`))
            (:`  `
              (set `self.Temp Position` _result_2)))))
      (if (== _array_element_2 _array_element_3)
        (set `self.isOwnPlayer` true)
        (else
          (set `self.isOwnPlayer` false)))
      (`/Game/Blueprints/TDMPlayerController.AddPlayerToSCoreboard` _astdmplayer_controller_2 (`self.isOwnPlayer`) (`AdvancedSessionsLibrary.GetPlayerName` _astdmplayer_controller_3) (`/Game/Blueprints/TDMPlayerController.Kills` _astdmplayer_controller_3) (`/Game/Blueprints/TDMPlayerController.Deaths` _astdmplayer_controller_3) (`self.Temp Position`) (`/Game/Blueprints/TDMPlayerController.SelectedTeam` _astdmplayer_controller_3)))))

(event `self.K2_OnLogout`
  (params (ExitingController :type "Controller Object Reference"))
  (bind _pcs (`self.PCs`))
  ;[1 0.2672 0.3369] PlayerList
  (for (_array_element _array_index) _pcs
    (if (== _array_element ExitingController)
      (break)))
  (`KismetArrayLibrary.Array_Remove` _pcs _array_index)
  (`self.UpdateServer`))

(event `UpdateScore`
  (params (Selection :type Integer))
  ;[0.09783 1 0.5293] Scoreboard
  (switch `int` Selection
    (:`1`
      (`/Engine/EditorBlueprintResources/StandardMacros.IncrementInt` (`self.TeamOneKillsNumber`)
        (:`  `
          _)))
    (:`2`
      (`/Engine/EditorBlueprintResources/StandardMacros.IncrementInt` (`self.TeamTwoKillsNumber`)
        (:`  `
          _))))
  (for _array_element (`self.PCs`)
    (bind _astdmplayer_controller (cast `/Game/Blueprints/TDMPlayerController` _array_element))
    (switch `int` Selection
      (:`1`
        (`/Game/Blueprints/TDMPlayerController.UpdateSCore` _astdmplayer_controller (`self.TeamOneKillsNumber`) Selection false (`self.TeamOneRoundNumber`)))
      (:`2`
        (`/Game/Blueprints/TDMPlayerController.UpdateSCore` _astdmplayer_controller (`self.TeamTwoKillsNumber`) Selection false (`self.TeamTwoRoundNumber`))))
    (if (>= (`self.TeamOneKillsNumber`) 50)
      (`/Game/Blueprints/TDMPlayerController.ShowEndGameWidget` _astdmplayer_controller "Team One Won!" 1)
      (`KismetSystemLibrary.Delay` 3.0 :!label _label)
      (`self.RestartRound`)
      (elif (>= (`self.TeamTwoKillsNumber`) 50)
        (`/Game/Blueprints/TDMPlayerController.ShowEndGameWidget` _astdmplayer_controller "Team Two Won!" 2)
        (goto _label))))
  (if (>= (`self.TeamOneKillsNumber`) 50)
    (set `self.TeamOneKillsNumber` 0)
    (set `self.TeamTwoKillsNumber` 0)
    (`/Engine/EditorBlueprintResources/StandardMacros.IncrementInt` (`self.TeamOneRoundNumber`)
      (:`  `
        (for _array_element_2 (`self.PCs`) :!label _label_2
          (bind _astdmplayer_controller_2 (cast `/Game/Blueprints/TDMPlayerController` _array_element_2))
          (switch `int` Selection
            (:`1`
              (`/Game/Blueprints/TDMPlayerController.UpdateSCore` _astdmplayer_controller_2 0 1 true (`self.TeamOneRoundNumber`)))
            (:`2`
              (`/Game/Blueprints/TDMPlayerController.UpdateSCore` _astdmplayer_controller_2 0 2 true (`self.TeamTwoRoundNumber`)))))))
    (elif (>= (`self.TeamTwoKillsNumber`) 50)
      (set `self.TeamOneKillsNumber` 0)
      (set `self.TeamTwoKillsNumber` 0)
      (`/Engine/EditorBlueprintResources/StandardMacros.IncrementInt` (`self.TeamTwoRoundNumber`)
        (:`  `
          (goto _label_2))))))

(event `KickPlayer`
  (params (Index :type Integer))
  ;[1 0.2672 0.3369] PlayerList
  (bind _astdmplayer_controller (cast `/Game/Blueprints/TDMPlayerController` (`|GetArrayItem` (`self.PCs`) Index)))
  (`/Game/Blueprints/TDMPlayerController.KickPlayer` _astdmplayer_controller))

(event `UpdateServer`
  (bind _isfail (`self.isFail`))
  (bind _returnvalue (`KismetArrayLibrary.Array_Length` (`self.PCs`)))
  ;[1 0.2672 0.3369] PlayerList
  (if (> _returnvalue (`self.MaxSlots`))
    (`self.KickPlayer` (- _returnvalue 1))
    (`KismetSystemLibrary.Delay` 0.2))
  (for _array_element (`self.PCs`)
    (bind _astdmplayer_controller (cast `/Game/Blueprints/TDMPlayerController` _array_element))
    (`/Game/Blueprints/TDMPlayerController.ClearPlayerList` _astdmplayer_controller)
    (for (_array_element_2 _array_index) (`self.PCs`)
      (bind _returnvalue_2 (`AdvancedSteamFriendsLibrary.GetSteamFriendAvatar` (`AdvancedSessionsLibrary.GetUniqueNetID` _array_element_2))
        (:`OnSuccess`
          (set `self.isFail` false))
        (:`AsyncLoading`
          (set `self.isFail` true))
        (:`OnFailure`
          (set `self.isFail` true)))
      (bind _astdmplayer_controller_2 (cast `/Game/Blueprints/TDMPlayerController` _array_element_2 :!pure true))
      (bind _returnvalue_3 (== (`/Game/Blueprints/TDMPlayerController.SelectedTeam` _astdmplayer_controller_2) 1))
      (if _returnvalue_3
        (bind _returnvalue_4 (`KismetTextLibrary.Conv_StringToText` (`AdvancedSessionsLibrary.GetPlayerName` _array_element_2)))
        (`/Game/Blueprints/TDMPlayerController.AddPlayerToTeamOne` _astdmplayer_controller _isfail _returnvalue_4 _returnvalue_2 _array_index (`KismetMathLibrary.SelectColor` (struct :`R` 1.0 :`G` 0.976471 :`B` 0.25098 :`A` 1.0) (struct :`R` 1.0 :`G` 1.0 :`B` 1.0 :`A` 1.0) _returnvalue_3))
        (else
          (bind _returnvalue_5 (== (`/Game/Blueprints/TDMPlayerController.SelectedTeam` _astdmplayer_controller_2) 2))
          (if _returnvalue_5
            (`/Game/Blueprints/TDMPlayerController.AddPlayerToTeamTwo` _astdmplayer_controller _isfail _returnvalue_4 _returnvalue_2 _array_index (`KismetMathLibrary.SelectColor` (struct :`R` 0.003922 :`B` 0.384314 :`A` 1.0) (struct :`R` 1.0 :`G` 1.0 :`B` 1.0 :`A` 1.0) _returnvalue_5))
            (else
              (`/Game/Blueprints/TDMPlayerController.AddPlayerToMainList` _astdmplayer_controller _isfail _returnvalue_4 _returnvalue_2 _array_index (struct :`R` 1.0 :`G` 1.0 :`B` 1.0 :`A` 1.0))))))))
  (for _array_element_3 (`self.PCs`)
    (bind _astdmplayer_controller_3 (cast `/Game/Blueprints/TDMPlayerController` _array_element_3))
    (`/Game/Blueprints/TDMPlayerController.UpdateNumberOfPlayers` _astdmplayer_controller_3 (`KismetArrayLibrary.Array_Length` (`self.PCs`)))))

(event `self.ReceiveBeginPlay`
  ;[0.4546 0.7407 1] DefaultEvents
  (bind _asmain_game_instance (cast `/Game/Blueprints/MainGameInstance` (`GameplayStatics.GetGameInstance`)))
  (set `self.Server Name` (`/Game/Blueprints/MainGameInstance.ServerName` _asmain_game_instance))
  (set `self.Map Name` (`/Game/Blueprints/MainGameInstance.ServerMap` _asmain_game_instance))
  (set `self.MaxSlots` (`/Game/Blueprints/MainGameInstance.ServerMaxPlayers` _asmain_game_instance)))

(event `self.K2_PostLogin`
  (params (NewPlayer :type "PlayerController Object Reference"))
  ;[0.4546 0.7407 1] DefaultEvents
  (`/Engine/EditorBlueprintResources/ActorMacros.Switch Has Authority`
    (:`Authority`
      (`KismetArrayLibrary.Array_Add` (`self.PCs`) NewPlayer)
      (`KismetSystemLibrary.Delay` 1.0)
      (`self.UpdateServer`)
      (`self.SetServerData` NewPlayer)
      (`KismetSystemLibrary.Delay` (`KismetMathLibrary.RandomFloatInRange` 0.1 1.0))
      (`self.UpdateServer`))))

(event `SetGameStatus`
  (params (CurrentStatus :type Boolean))
  (set `self.IsGameGoing` CurrentStatus)
  (bind _asmain_game_instance (cast `/Game/Blueprints/MainGameInstance` (`GameplayStatics.GetGameInstance`)))
  (`/Game/Blueprints/MainGameInstance.UpdateGameStatus` _asmain_game_instance CurrentStatus))

(event `SetServerData`
  (params (CurrentPC :type "PlayerController Object Reference"))
  ;[1 0.9979 0.3372] ServerData
  (bind _astdmplayer_controller (cast `/Game/Blueprints/TDMPlayerController` CurrentPC))
  (`/Game/Blueprints/TDMPlayerController.UpdateServerData` _astdmplayer_controller (`KismetTextLibrary.Conv_StringToText` (`self.Map Name`)) (`KismetTextLibrary.Conv_StringToText` (`self.Server Name`)) (`self.MaxSlots`)))

(event `JoinGame`
  (params (PC :type "PlayerController Object Reference"))
  (bind _astdmplayer_controller (cast `/Game/Blueprints/TDMPlayerController` PC :!pure true))
  (bind _selectedteam (`/Game/Blueprints/TDMPlayerController.SelectedTeam` _astdmplayer_controller))
  ;[1 0.4812 0.3102] Start/Restart GameThings
  (switch `int` _selectedteam
    (:`1`
      (`KismetArrayLibrary.Array_Add` (`self.TeamOnePCs`) PC)
      (bind _outactors (`GameplayStatics.GetAllActorsOfClass` "/Game/Blueprints/TeamOneSpawnPoint.TeamOneSpawnPoint_C"))
      (bind _returnvalue_location (`KismetMathLibrary.BreakTransform` (`self.GetTransform` (`|GetArrayItem` _outactors (`KismetMathLibrary.RandomInteger` (`KismetArrayLibrary.Array_Length` _outactors))))))
      (bind _returnvalue (`|SpawnActorFromClass` "/Game/Blueprints/Characters/Character_TeamOne.Character_TeamOne_C" (`KismetMathLibrary.MakeTransform` _returnvalue_location) "Undefined" "OverrideRootScale" null _selectedteam null))
      (`Controller.Possess` _astdmplayer_controller _returnvalue))
    (:`2`
      (`KismetArrayLibrary.Array_Add` (`self.TeamTwoPCs`) PC)
      (bind _outactors_2 (`GameplayStatics.GetAllActorsOfClass` "/Game/Blueprints/TeamTwoSpawnPoint.TeamTwoSpawnPoint_C"))
      (bind _returnvalue_location_2 (`KismetMathLibrary.BreakTransform` (`self.GetTransform` (`|GetArrayItem` _outactors_2 (`KismetMathLibrary.RandomInteger` (`KismetArrayLibrary.Array_Length` _outactors_2))))))
      (bind _returnvalue_2 (`|SpawnActorFromClass` "/Game/Blueprints/Characters/Character_TeamTwo.Character_TeamTwo_C" (`KismetMathLibrary.MakeTransform` _returnvalue_location_2) "Undefined" "OverrideRootScale" null _selectedteam null))
      (`Controller.Possess` _astdmplayer_controller _returnvalue_2)))
  (`self.UpdateScoreboard`)
  (bind _asmain_game_instance (cast `/Game/Blueprints/MainGameInstance` (`GameplayStatics.GetGameInstance`)))
  (`/Game/Blueprints/MainGameInstance.JoinGame` _asmain_game_instance))

(event `RestartRound`
  (bind _spawnpointsindexone (`self.SpawnPointsIndexOne`))
  (bind _spawnpointsindextwo (`self.SpawnPointsIndexTwo`))
  ;[1 0.4812 0.3102] Start/Restart GameThings
  (set `self.SpawnPointsIndexOne` 0)
  (set `self.SpawnPointsIndexTwo` 0)
  (for _array_element (`self.PCs`)
    (bind _astdmplayer_controller (cast `/Game/Blueprints/TDMPlayerController` _array_element))
    (switch `int` (`/Game/Blueprints/TDMPlayerController.SelectedTeam` _astdmplayer_controller)
      (:`1`
        (bind _outactors (`GameplayStatics.GetAllActorsOfClass` "/Game/Blueprints/TeamOneSpawnPoint.TeamOneSpawnPoint_C"))
        (`/Engine/EditorBlueprintResources/StandardMacros.IncrementInt` _spawnpointsindexone
          (:`  `
            (bind _returnvalue (`Controller.K2_GetPawn` _astdmplayer_controller))
            (`self.K2_SetActorTransform` _returnvalue (`self.GetTransform` (`|GetArrayItem` _outactors _spawnpointsindexone)) false false))))
      (:`2`
        (bind _outactors_2 (`GameplayStatics.GetAllActorsOfClass` "/Game/Blueprints/TeamTwoSpawnPoint.TeamTwoSpawnPoint_C"))
        (`/Engine/EditorBlueprintResources/StandardMacros.IncrementInt` _spawnpointsindextwo
          (:`  `
            (`self.K2_SetActorTransform` _returnvalue (`self.GetTransform` (`|GetArrayItem` _outactors_2 _spawnpointsindextwo)) false false))))))
  (if (or (>= (`self.TeamOneRoundNumber`) 2) (>= (`self.TeamTwoRoundNumber`) 2))
    (set `self.TeamOneRoundNumber` 0)
    (set `self.TeamTwoRoundNumber` 0)
    (bind _outactors_3 (`GameplayStatics.GetAllActorsOfClass` "/Game/Blueprints/Characters/FirstPersonCharacter.FirstPersonCharacter_C"))
    (for _array_element_2 _outactors_3
      (`self.K2_DestroyActor` _array_element_2))
    (for _array_element_3 (`self.PCs`)
      (bind _astdmplayer_controller_2 (cast `/Game/Blueprints/TDMPlayerController` _array_element_3))
      (set `/Game/Blueprints/TDMPlayerController.Kills` 0 _astdmplayer_controller_2)
      (set `/Game/Blueprints/TDMPlayerController.Deaths` 0 _astdmplayer_controller_2)
      (set `/Game/Blueprints/TDMPlayerController.UsingWEapon` "NewEnumerator0" _astdmplayer_controller_2)
      (`/Game/Blueprints/TDMPlayerController.UpdateSCore` _astdmplayer_controller_2 0 1 true 0)
      (`/Game/Blueprints/TDMPlayerController.UpdateSCore` _astdmplayer_controller_2 0 2 true 0)
      (`/Game/Blueprints/TDMPlayerController.ShowLobbyWidget` _astdmplayer_controller_2)
      (`self.SetGameStatus` false))))

(fn `UserConstructionScript`)