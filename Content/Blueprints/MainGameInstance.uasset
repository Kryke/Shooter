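; Game instance Blueprint that handles multiplayer session hosting and invite acceptance.
; CreateSession stores server settings, creates an advanced session with name, map, LAN and status properties, then opens MainMap as a listen server.
; UpdateGameStatus republishes those properties with the new in-game status, allowing invites and join-in-progress.
; Accepted invites join directly, while JoinGame is an empty stub marked for rework and DestroySession is unwired.
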(event `self.OnSessionInviteAccepted`
  (params (LocalPlayerNum :type Integer) (PersonInvited :type "BPUniqueNetId Structure") (SessionToJoin :type "BlueprintSessionResult Structure (by ref)"))
  ;[1 1 1] Invite
  (`JoinSessionCallbackProxy.JoinSession` (`GameplayStatics.GetPlayerController` 0) SessionToJoin))

(event `JoinGame`
  ;[1 1 1] Need Rework
)

(event `Create Session`
  (params (ServerName :type String) (ServerMap :type String) (ServerSlots :type Integer) (IsServerMethodLan :type Boolean))
  ;[1 1 1] Creating/Updating Session
  (set `self.ServerName` ServerName)
  (set `self.ServerMap` ServerMap)
  (set `self.ServerMaxPlayers` ServerSlots)
  (set `self.IsServerMethodLan` IsServerMethodLan)
  (`CreateSessionCallbackProxyAdvanced.CreateAdvancedSession` (`|MakeArray` (`AdvancedSessionsLibrary.MakeLiteralSessionPropertyString` "ServerName" (`self.ServerName`)) (`AdvancedSessionsLibrary.MakeLiteralSessionPropertyString` "ServerMap" (`self.ServerMap`)) (`AdvancedSessionsLibrary.MakeLiteralSessionPropertyBool` "IsLan" (`self.IsServerMethodLan`)) (`AdvancedSessionsLibrary.MakeLiteralSessionPropertyBool` "Status" (`self.IsGameGoing`))) (`GameplayStatics.GetPlayerController` 0) (`self.ServerMaxPlayers`) 0 (`self.IsServerMethodLan`)
    (:`OnSuccess`
      (`GameplayStatics.OpenLevel` "MainMap" true "listen"))))

(event `UpdateGameStatus`
  (params (InGameStatus :type Boolean))
  ;[1 1 1] Creating/Updating Session
  (set `self.IsGameGoing` InGameStatus)
  (`UpdateSessionCallbackProxyAdvanced.UpdateSession` (`|MakeArray` (`AdvancedSessionsLibrary.MakeLiteralSessionPropertyString` "ServerName" (`self.ServerName`)) (`AdvancedSessionsLibrary.MakeLiteralSessionPropertyString` "ServerMap" (`self.ServerMap`)) (`AdvancedSessionsLibrary.MakeLiteralSessionPropertyBool` "IsLan" (`self.IsServerMethodLan`)) (`AdvancedSessionsLibrary.MakeLiteralSessionPropertyBool` "Status" (`self.IsGameGoing`))) (`self.ServerMaxPlayers`) 0 (`self.IsServerMethodLan`) true true))