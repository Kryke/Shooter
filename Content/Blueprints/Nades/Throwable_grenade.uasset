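; Throwable grenade actor that launches itself from the player's view and leaves a FlashDecal when its fuse ends.
; On BeginPlay, it applies an impulse to its mesh along the first-person camera's forward vector.
; After a fixed delay, it spawns the FlashDecal at the mesh's current location with a fixed rotation, then destroys itself.
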(event `self.ReceiveBeginPlay`
  (bind _asfirst_person_character (cast `/Game/Blueprints/Characters/FirstPersonCharacter` (`GameplayStatics.GetPlayerPawn` 0)))
  (`PrimitiveComponent.AddImpulse` (`self.ThrowableMesh`) (* (`SceneComponent.GetForwardVector` (`/Game/Blueprints/Characters/FirstPersonCharacter.FirstPersonCamera` _asfirst_person_character)) 2000.0) "None" false)
  (`KismetSystemLibrary.Delay` 4.0)
  (`|SpawnActorFromClass` "/Game/Blueprints/Nades/FlashDecal.FlashDecal_C" (`KismetMathLibrary.MakeTransform` (`SceneComponent.K2_GetComponentLocation` (`self.ThrowableMesh`)) (struct :`Pitch` 90.0)) "Undefined" "OverrideRootScale" null null)
  (`self.K2_DestroyActor`))

(fn `UserConstructionScript`)