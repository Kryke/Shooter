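; Throwable flashbang grenade actor that launches itself from the player's view and detonates on a timer.
; On BeginPlay it applies an impulse to the Flashnade component along the first-person camera's forward vector.
; After a short delay it spawns a flash decal at the grenade's position, passes horizontal distance and grenade location to the player character's FlashEffect, then destroys itself.
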(event `self.ReceiveBeginPlay`
  (bind _returnvalue (`SceneComponent.K2_GetComponentLocation` (`self.flashnade`)))
  (bind _asfirst_person_character (cast `/Game/Blueprints/Characters/FirstPersonCharacter` (`GameplayStatics.GetPlayerPawn` 0)))
  (`PrimitiveComponent.AddImpulse` (`self.flashnade`) (* (`SceneComponent.GetForwardVector` (`/Game/Blueprints/Characters/FirstPersonCharacter.FirstPersonCamera` _asfirst_person_character)) 2000.0) "None" false)
  (`KismetSystemLibrary.Delay` 4.0)
  (`|SpawnActorFromClass` "/Game/Blueprints/Nades/FlashDecal.FlashDecal_C" (`KismetMathLibrary.MakeTransform` _returnvalue (struct :`Pitch` 90.0)) "Undefined" "OverrideRootScale" null null)
  (`/Game/Blueprints/Characters/FirstPersonCharacter.FlashEffect` _asfirst_person_character (`self.GetHorizontalDistanceTo` _asfirst_person_character) _returnvalue)
  (`self.K2_DestroyActor`))

(event `self.ThrowableMesh.OnComponentHit`
  (params (HitComponent :type "PrimitiveComponent Object Reference") (OtherActor :type "Actor Object Reference") (OtherComp :type "PrimitiveComponent Object Reference") (NormalImpulse :type "Vector Structure") (Hit :type "HitResult Structure (by ref)")))

(fn `UserConstructionScript`)