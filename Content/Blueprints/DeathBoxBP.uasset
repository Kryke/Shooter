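; DeathBoxBP is a lootable box actor that holds bullets and destroys itself after a fixed delay from BeginPlay.
; When a FirstPersonCharacter enters its sphere, it adds an Ammo entry with the bullet count and a self reference to the loot list in that player's TDMPlayerController HUD, unless empty.
; Leaving the sphere clears that loot list.
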(event `self.ReceiveBeginPlay`
  (`KismetSystemLibrary.Delay` 40.0)
  (`self.K2_DestroyActor`))

(event `self.ReceiveTick`
  (params (DeltaSeconds :type "Float (single-precision)")))

(event `self.Sphere.OnComponentBeginOverlap`
  (params (OverlappedComponent :type "PrimitiveComponent Object Reference") (OtherActor :type "Actor Object Reference") (OtherComp :type "PrimitiveComponent Object Reference") (OtherBodyIndex :type Integer) (bFromSweep :type Boolean) (SweepResult :type "HitResult Structure (by ref)"))
  (bind _asfirst_person_character (cast `/Game/Blueprints/Characters/FirstPersonCharacter` OtherActor))
  (bind _astdmplayer_controller (cast `/Game/Blueprints/TDMPlayerController` (`Pawn.GetController` _asfirst_person_character)))
  (if (not (== (`self.Bullets`) 0))
    (`/Game/UI/Gameplay/UMG_LootListBox.AddItemToBox` (`/Game/UI/HUD/UMG_PlayerHUD.UMG_LootListBox` (`/Game/Blueprints/TDMPlayerController.HUDWIdget` _astdmplayer_controller)) "Ammo" (`self.Bullets`) "NewEnumerator0" self "NewEnumerator0")))

(event `self.Sphere.OnComponentEndOverlap`
  (params (OverlappedComponent :type "PrimitiveComponent Object Reference") (OtherActor :type "Actor Object Reference") (OtherComp :type "PrimitiveComponent Object Reference") (OtherBodyIndex :type Integer))
  (bind _asfirst_person_character (cast `/Game/Blueprints/Characters/FirstPersonCharacter` OtherActor))
  (bind _astdmplayer_controller (cast `/Game/Blueprints/TDMPlayerController` (`Pawn.GetController` _asfirst_person_character)))
  (`/Game/UI/Gameplay/UMG_LootListBox.ClearItems` (`/Game/UI/HUD/UMG_PlayerHUD.UMG_LootListBox` (`/Game/Blueprints/TDMPlayerController.HUDWIdget` _astdmplayer_controller))))

(fn `UserConstructionScript`)