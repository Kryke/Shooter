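; Player camera manager that drives the first-person view while aiming down sights.
; BlueprintUpdateCamera takes pitch and yaw from the weapon's Ironsight-to-Muzzle line, with zero roll and no blending.
; Location blends from the character camera to the sight socket chosen by the controller's UsingScope, nudged along the sight axis by a scaled camera-to-socket projection.
; ADSTrack drives that blend and narrows FOV; the override applies only while IsADSing.
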(fn `BlueprintUpdateCamera`
  (params (CameraTarget :type "Actor Object Reference"))
  (returns (NewCameraLocation :type "Vector Structure") (NewCameraRotation :type "Rotator Structure") (NewCameraFOV :type "Float (double-precision)") (ReturnValue :type Boolean))
  (locals (NewLocalVar_0 :type "Rotator Structure" :default (struct)))
  (bind _player (`self.Player`))
  (bind _returnvalue (`SceneComponent.K2_GetComponentLocation` (`/Game/Blueprints/Characters/FirstPersonCharacter.FirstPersonCamera` _player)))
  (bind _weaponmesh (`/Game/Blueprints/Weapon/Weapon_Base_BP.WeaponMesh` (`/Game/Blueprints/Characters/FirstPersonCharacter.UsingWEapon` (`self.Player`))))
  (bind _weaponmesh_2 (`/Game/Blueprints/Weapon/Weapon_Base_BP.WeaponMesh` (`/Game/Blueprints/Characters/FirstPersonCharacter.UsingWEapon` _player)))
  (bind _returnvalue_2 (`SceneComponent.GetSocketTransform` _weaponmesh_2 "Ironsight" "RTS_World"))
  (bind _returnvalue_location (`KismetMathLibrary.BreakTransform` (`SceneComponent.GetSocketTransform` _weaponmesh "Muzzle" "RTS_World")))
  (bind _returnvalue_location_2 (`KismetMathLibrary.BreakTransform` (`SceneComponent.GetSocketTransform` _weaponmesh "Ironsight" "RTS_World")))
  (bind (_returnvalue_roll _returnvalue_pitch _returnvalue_yaw) (`KismetMathLibrary.BreakRotator` (`KismetMathLibrary.FindLookAtRotation` _returnvalue_location_2 _returnvalue_location)))
  (bind _location (.location (select `/Game/Blueprints/Enums-Structs/Scopes` (`/Game/Blueprints/TDMPlayerController.UsingScope` (cast `/Game/Blueprints/TDMPlayerController` (`Pawn.GetController` _player) :!pure true)) :`NewEnumerator0` _returnvalue_2 :`NewEnumerator1` (`SceneComponent.GetSocketTransform` _weaponmesh_2 "IronsightScope" "RTS_World") :`NewEnumerator2` _returnvalue_2)))
  (bind _returnvalue_3 (`KismetMathLibrary.GetForwardVector` (.rotation (select `/Game/Blueprints/Enums-Structs/Scopes` (`/Game/Blueprints/TDMPlayerController.UsingScope` (cast `/Game/Blueprints/TDMPlayerController` (`Pawn.GetController` _player) :!pure true)) :`NewEnumerator0` _returnvalue_2 :`NewEnumerator1` (`SceneComponent.GetSocketTransform` _weaponmesh_2 "IronsightScope" "RTS_World") :`NewEnumerator2` _returnvalue_2))))
  (bind _returnvalue_4 (- _location _returnvalue))
  (bind _asfirst_person_character (cast `/Game/Blueprints/Characters/FirstPersonCharacter` CameraTarget))
  (bind _output_get (set `self.Player` _asfirst_person_character))
  (`/Engine/EditorBlueprintResources/StandardMacros.IsValid` _output_get
    (:`Is Valid`
      (if (`/Game/Blueprints/Characters/FirstPersonCharacter.IsADSing` (`self.Player`))
        (set `self.ADS Camera Rotation` (`KismetMathLibrary.MakeRotator` 0.0 _returnvalue_pitch _returnvalue_yaw))
        (set `self.ADS Camera Location` (`KismetMathLibrary.VLerp` _returnvalue (- _location (* _returnvalue_3 (* (`KismetMathLibrary.Dot_VectorVector` (`KismetMathLibrary.Normal` _returnvalue_4 0.0) _returnvalue_3) (/ (`KismetMathLibrary.VSize` _returnvalue_4) 250.0)))) (`/Game/Blueprints/Characters/FirstPersonCharacter.ADSTrack` (`self.Player`))))
        (return (`self.ADS Camera Location`) (`self.ADS Camera Rotation`) (`KismetMathLibrary.Lerp` 103.0 80.0 (`/Game/Blueprints/Characters/FirstPersonCharacter.ADSTrack` (`self.Player`))) true)))))

(fn `UserConstructionScript`)